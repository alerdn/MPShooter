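; Player controller for the multiplayer shooter, handling the local HUD, pause menu, death and respawn.
; Pawn death is reported to the GameMode, then the body is unpossessed and destroyed after a delay, triggering respawn at a random PlayerStart and event rebinding.
; Player-list and notification events retry until the HUD is valid, and name changes refresh the list through the GameMode.
; Pausing only switches input and shows the menu.
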(event `On Player Spawn`
  ;[1 1 1] On Player Spawn
  (bind _asbp_mpshooter_character (cast `/Game/Blueprints/Character/BP_MPShooterCharacter` (`self.K2_GetPawn`) :!label _label))
  (`|ExecutionSequence`
    (:`then_0`
      (add `MPShooterCharacter.OnDead` _asbp_mpshooter_character (delegate `OnDead_Event`)))
    (:`then_1`
      (add `self.OnDestroyed` _asbp_mpshooter_character (delegate `OnDestroyed_Event`)))
    (:`then_2`
      (add `self.OnPlayerNameChanged` (delegate `OnPlayerNameChanged_Event`)))))

(event `self.ReceiveBeginPlay`
  (if (`self.IsLocalController`)
    ;[1 1 1] Init
    (`self.InitUI`)))

(event `OnDead_Event`
  (params (Player :type "MPShooterCharacter Object Reference") (Killer :type "MPShooterCharacter Object Reference") (Weapon :type "Gun Object Reference"))
  ;[1 1 1] On Player Spawn
  (bind _asbp_mpshooter_game_mode (cast `/Game/Blueprints/GameModes/BP_MPShooterGameMode` (`GameplayStatics.GetGameMode`)))
  (`/Game/Blueprints/GameModes/BP_MPShooterGameMode.On Dead` _asbp_mpshooter_game_mode Player Killer Weapon self)
  (`self.UnPossess`)
  (`KismetSystemLibrary.Delay` 5.0)
  (`self.K2_DestroyActor` Player))

(event `Key|Escape`
  (params (Key :type "Key Structure"))
  ;[1 1 1] Pause
  (:`Pressed`
    (if (`self.IsPaused`)
      (`self.Un Pause Game`)
      (else
        (`self.Pause Game`)))))

(event `OnDestroyed_Event` :!signature `self.OnDestroyed`
  (params (DestroyedActor :type "Actor Object Reference"))
  ;[1 1 1] On Player Spawn
  (`GameModeBase.RestartPlayerAtPlayerStart` (`GameplayStatics.GetGameMode`) self (`self.GetRandomPlayerStart`))
  (goto _label))

(event `On Player List Updated`
  (params (PlayersData :type "Array of /Game/Blueprints/Character/ST_Player Structure"))
  (bind _hud (`self.HUD`))
  ;[1 1 1] Update Player List
  (`/Engine/EditorBlueprintResources/StandardMacros.IsValid` _hud :!label _label_2
    (:`Is Valid`
      (`/Game/Blueprints/UI/WBP_HUD.Update Player List` _hud PlayersData))
    (:`Is Not Valid`
      (`KismetSystemLibrary.Delay` 0.1)
      (goto _label_2))))

(event `Key|Tab`
  (params (Key :type "Key Structure"))
  (bind _hud (`self.HUD`))
  ;[1 1 1] Toggle Player List
  (:`Pressed`
    (`/Game/Blueprints/UI/WBP_HUD.Show Player List` _hud true))
  (:`Released`
    (`/Game/Blueprints/UI/WBP_HUD.Show Player List` _hud false)))

(event `OnPlayerNameChanged_Event`
  ;[1 1 1] On Player Spawn
  (bind _asbp_mpshooter_game_mode (cast `/Game/Blueprints/GameModes/BP_MPShooterGameMode` (`GameplayStatics.GetGameMode`)))
  (`/Game/Blueprints/GameModes/BP_MPShooterGameMode.Update Player List` _asbp_mpshooter_game_mode))

(event `On Notification`
  (params (Notification :type Text))
  (bind _hud (`self.HUD`))
  ;[1 1 1] Add Notification
  (`/Engine/EditorBlueprintResources/StandardMacros.IsValid` _hud :!label _label_3
    (:`Is Valid`
      (`/Game/Blueprints/UI/WBP_HUD.Add Notification` _hud Notification))
    (:`Is Not Valid`
      (`KismetSystemLibrary.Delay` 0.1)
      (goto _label_3))))

(fn `GetRandomPlayerStart`
  (returns (PlayerStart :type "PlayerStart Object Reference"))
  (bind _outactors (`GameplayStatics.GetAllActorsOfClass` "/Script/Engine.PlayerStart"))
  (return (`KismetArrayLibrary.Array_Random` _outactors)))

(fn `InitUI`
  (bind _returnvalue (`|CreateWidget` "/Game/Blueprints/UI/WBP_HUD.WBP_HUD_C"))
  (bind _output_get (set `self.HUD` _returnvalue))
  (`UserWidget.AddToViewport` _output_get 0)
  (bind _returnvalue_2 (`|CreateWidget` "/Game/Blueprints/UI/WBP_PauseMenu.WBP_PauseMenu_C"))
  (set `self.Menu Widget` _returnvalue_2)
  (set `self.IsPaused` false))

(fn `Pause Game`
  (if (`self.IsLocalPlayerController`)
    (`UserWidget.AddToViewport` (`self.Menu Widget`) 0)
    (`WidgetBlueprintLibrary.SetInputMode_UIOnlyEx` self null)
    (`self.SetIgnoreLookInput` self true)
    (set `self.bShowMouseCursor` true)
    (set `self.IsPaused` true)))

(fn `Un Pause Game`
  (if (`self.IsLocalPlayerController`)
    (`Widget.RemoveFromParent` (`self.Menu Widget`))
    (`WidgetBlueprintLibrary.SetInputMode_GameOnly` self)
    (`self.ResetIgnoreLookInput` self)
    (set `self.bShowMouseCursor` false)
    (set `self.IsPaused` false)))

(fn `UserConstructionScript`)