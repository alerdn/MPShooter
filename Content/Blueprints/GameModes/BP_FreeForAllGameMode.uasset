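; Free-for-all game mode for a multiplayer shooter, with a match won by reaching a kill target.
; VerifyWinCondition compares the killer's kill count to KillToWin, sets MatchEnded, prints the winner's name, then reloads the level after a delay.
; OnDead extends the parent handler and, while the match runs, casts the killer's controller to MPShooterPlayerController, with no further action wired.
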(event `self.ReceiveBeginPlay`
  (set `self.MatchEnded` false))

(event `Verify Win Condition`
  (params (KillerController :type "MPShooterPlayerController Object Reference"))
  (if (>= (`MPShooterPlayerController.GetKillsCount` KillerController) (`self.KillToWin`))
    (set `self.MatchEnded` true)
    (`KismetSystemLibrary.PrintString` (`KismetStringLibrary.Concat_StrStr` (`MPShooterPlayerController.GetPlayerName` KillerController) " venceu!!!") true true (struct :`G` 0.66 :`B` 1.0 :`A` 1.0) 10.0)
    (`KismetSystemLibrary.Delay` 10.0)
    (`self.ReloadLevel`)))

(fn `On Dead`
  (params (Killer :type "MPShooterCharacter Object Reference") (Weapon :type "Gun Object Reference") (PlayerController :type "MPShooterPlayerController Object Reference"))
  (`parent.On Dead` Killer Weapon PlayerController)
  (if (not (`self.MatchEnded`))
    (cast `MPShooterPlayerController` (`Pawn.GetController` Killer))))

(fn `UserConstructionScript`
  (`parent.UserConstructionScript`))